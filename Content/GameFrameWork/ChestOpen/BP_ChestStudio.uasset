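; BP_ChestStudio is a capture-studio actor that presents an animated chest for a chest-opening sequence.
; StartIntroSequence plays the skeletal chest's intro animation once, then switches to looping idle after a fixed delay.
; StartOpenSequence plays the open animation once.
; The construction script adds the actor's own components, child actors included, to its SceneCaptureComponent2D show-only list to isolate the chest in the capture.
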(event Custom|StartOpenSequence
  (Components|Animation|PlayAnimation (Variables|Default|GetChestSkel) "/Game/External_Asset/Animator/B_ChestRigged__23390/B_ChestRigged_Anim_Open.B_ChestRigged_Anim_Open" false))

(event Custom|StartIntroSequence
  (bind _chestskel (Variables|Default|GetChestSkel))
  (Components|Animation|PlayAnimation _chestskel "/Game/External_Asset/Animator/B_ChestRigged__23390/B_ChestRigged_Anim_Intro.B_ChestRigged_Anim_Intro" false)
  (Utilities|FlowControl|Delay 1.0)
  (Components|Animation|PlayAnimation _chestskel "/Game/External_Asset/Animator/B_ChestRigged__23390/B_ChestRigged_Anim_Idle.B_ChestRigged_Anim_Idle" true))

(fn ConstructionScript
  (Rendering|SceneCapture|ShowOnlyActorComponents (Variables|Default|GetSceneCaptureComponent2D) self true))