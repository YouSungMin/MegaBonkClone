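; BP_TestEnemy2 is a test enemy Blueprint that deals and receives damage, logging both with Print String.
; On BeginPlay it binds to its OnTakeAnyDamage event and prints the amount of any damage it takes.
; When another actor overlaps it, it calls ApplyDamage on that actor using its BaseDamage variable and prints the returned value.
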(event Custom|OnTakeAnyDamage_Event
  (params (DamagedActor :type Actor%20Object%20Reference) (Damage :type Float%20%28single-precision%29) (DamageType :type Damage%20Type%20Object%20Reference) (InstigatedBy :type Controller%20Object%20Reference) (DamageCauser :type Actor%20Object%20Reference))
  (Development|PrintString (Utilities|String|ToString(Float) Damage)))

(event EventBeginPlay
  (|CallParentFunction)
  (EventDispatchers|BindEventtoOnTakeAnyDamage (delegate Custom|OnTakeAnyDamage_Event)))

(event Collision|EventActorBeginOverlap
  (params (OtherActor :type Actor%20Object%20Reference))
  (bind _returnvalue (Game|Damage|ApplyDamage OtherActor (Variables|Default|GetBase%20Damage) 0 0))
  (Development|PrintString (Utilities|String|ToString(Float) _returnvalue)))

(event EventTick
  (params (DeltaSeconds :type Float%20%28single-precision%29))
  (|CallParentFunction DeltaSeconds) ; 지금 이 노드는 비활성 상태입니다. \n핀을 끌어서 다른 노드를 연결하면 활성화됩니다.
)

(fn ConstructionScript
  (|CallParentFunction))