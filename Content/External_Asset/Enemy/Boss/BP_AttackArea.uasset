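; BP_AttackArea is an enemy boss area attack actor that telegraphs a spot, then strikes it with a rising mesh.
; On BeginPlay, the AreaGrowth timeline scales the Sphere indicator, which is destroyed when the timeline ends.
; The SpikeUp timeline then stretches AttackMesh along Z.
; When it finishes, BP_CharacterBase actors overlapping Sphere1 take BaseDamage in one hit, and the actor destroys itself after a short delay.
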(event EventBeginPlay
  (bind _scaletrack (Timeline|AreaGrowth Play)
    (:Update
      (Transformation|SetWorldScale3D (Variables|Default|GetSphere) (Math|Vector|MakeVector _scaletrack _scaletrack _scaletrack)))
    (:Finished
      (Components|DestroyComponent (Variables|Default|GetSphere))
      (bind _zscale (Timeline|SpikeUp Play)
        (:Update
          (Transformation|SetWorldScale3D (Variables|Default|GetAttackMesh) (Math|Vector|MakeVector 1.0 1.0 _zscale)))
        (:Finished
          (for _array_element (Collision|GetOverlappingActors (Variables|Default|GetSphere1) "/Game/Characters/PlayAbleCharacter/BP_CharacterBase.BP_CharacterBase_C" :!class /Script/Engine.PrimitiveComponent)
            (Game|Damage|ApplyDamage _array_element (Variables|Default|GetBase%20Damage) 0 0))
          (Utilities|FlowControl|Delay 0.5)
          (Actor|DestroyActor))))))

(event Collision|EventActorBeginOverlap
  (params (OtherActor :type Actor%20Object%20Reference)))

(event EventTick
  (params (DeltaSeconds :type Float%20%28single-precision%29)))

(fn ConstructionScript)