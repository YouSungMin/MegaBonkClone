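; Boss homing projectile that chases the player character and deals damage on contact.
; On BeginPlay it sets the player's BP_CharacterBase mesh as the ProjectileMovement homing target, then destroys itself after a timed lifetime.
; A sphere overlap with any BP_CharacterBase applies damage, hides the static mesh, activates Niagara and destroys the actor after a short delay.
; The lifetime timer only starts when a valid player character is found.
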(event OnComponentBeginOverlap(Sphere)
  (params (OverlappedComponent :type Primitive%20Component%20Object%20Reference) (OtherActor :type Actor%20Object%20Reference) (OtherComp :type Primitive%20Component%20Object%20Reference) (OtherBodyIndex :type Integer) (bFromSweep :type Boolean) (SweepResult :type Hit%20Result%20Structure%20%28by%20ref%29))
  (Utilities|Casting|CastToBP_CharacterBase OtherActor)
  (Game|Damage|ApplyDamage 0 (Variables|Default|GetBase%20Damage) 0 0)
  (Development|SetHiddeninGame (Variables|Default|GetStaticMesh) true false)
  (Components|Activation|Activate (Variables|Default|GetNiagara) true)
  (Utilities|FlowControl|Delay 1.0)
  (Actor|DestroyActor))

(event EventBeginPlay
  (bind _returnvalue (Game|GetPlayerCharacter 0))
  (Utilities|IsValid _returnvalue
    (:Is%20Valid
      (bind _asbp_character_base (Utilities|Casting|CastToBP_CharacterBase _returnvalue))
      (Variables|/Script/Engine.ProjectileMovementComponent|SetHomingTargetComponent (Variables|Default|GetProjectileMovement) (Variables|/Script/Engine.Character|GetMesh _asbp_character_base))
      (Utilities|FlowControl|Delay 1e+01)
      (Actor|DestroyActor))))

(fn ConstructionScript)