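; Base enemy actor that chases the player, deals contact damage and drops items on death.
; A DT_EnemyDataTable row sets speed, attack and max HP, with health raised by a Time-based bonus.
; AI MoveTo re-issues itself after each result, while sphere overlap runs a looping damage timer.
; At zero health it returns to BP_PoolManager under a fixed type, with activate/deactivate events toggling visibility and collision for reuse.
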(event OnComponentBeginOverlap(Sphere)
  (params (OverlappedComponent :type Primitive%20Component%20Object%20Reference) (OtherActor :type Actor%20Object%20Reference) (OtherComp :type Primitive%20Component%20Object%20Reference) (OtherBodyIndex :type Integer) (bFromSweep :type Boolean) (SweepResult :type Hit%20Result%20Structure%20%28by%20ref%29))
  (Utilities|Casting|CastToBP_CharacterBase OtherActor)
  (bind _returnvalue (Utilities|Time|SetTimerbyEvent (delegate Custom|DamageToPlayer) 1.0 true))
  (Variables|Default|SetDamageTimerHandle _returnvalue))

(event OnComponentEndOverlap(Sphere)
  (params (OverlappedComponent :type Primitive%20Component%20Object%20Reference) (OtherActor :type Actor%20Object%20Reference) (OtherComp :type Primitive%20Component%20Object%20Reference) (OtherBodyIndex :type Integer))
  (Utilities|Casting|CastToBP_CharacterBase OtherActor)
  (Utilities|Time|ClearandInvalidateTimerbyHandle (Variables|Default|GetDamageTimerHandle)))

(event Custom|MoveGoblin
  (AI|AIMoveTo self "0, 0, 0" (Game|GetPlayerCharacter 0) 5.0 false
    (:OnSuccess
      (Utilities|FlowControl|Delay 0.1)
      (CallFunction|MoveGoblin))
    (:OnFail
      (Utilities|FlowControl|Delay 0.1)
      (CallFunction|MoveGoblin))))

(event Custom|DamageToPlayer
  (Game|Damage|ApplyDamage (Game|GetPlayerCharacter 0) (.attackpower (stale EventBeginPlay _returnvalue)) 0 0))

(event EventBeginPlay
  (bind _returnvalue (Utilities|GetDataTableRow "/Game/Data/Enemy/DT_EnemyDataTable.DT_EnemyDataTable" (Variables|Default|GetRowName))
    (:then
      (CallFunction|MoveGoblin)
      (Variables|Default|SetHealth (+ (.maxhp _returnvalue) (/ (+ (Variables|Default|GetTime) (Utilities|Time|GetWorldDeltaSeconds)) 1e+01)))
      (Variables|/Script/Engine.CharacterMovementComponent|SetMaxWalkSpeed (Variables|Character|GetCharacterMovement) (.movespeed _returnvalue)))))

(event EventOnDeactivate
  (Rendering|SetActorHiddenInGame true)
  (Collision|SetActorEnableCollision false))

(event EventOnActivate
  (Rendering|SetActorHiddenInGame false)
  (Collision|SetActorEnableCollision true)
  (Variables|Default|SetHealth (+ (.maxhp (stale EventBeginPlay _returnvalue)) (/ (+ (Variables|Default|GetTime) (Utilities|Time|GetWorldDeltaSeconds)) 1e+01))))

(event Game|Damage|EventAnyDamage
  (params (Damage :type Float%20%28single-precision%29) (DamageType :type Damage%20Type%20Object%20Reference) (InstigatedBy :type Controller%20Object%20Reference) (DamageCauser :type Actor%20Object%20Reference))
  (Class|EnemyBase|ShowDamagePopup Damage)
  (Variables|Default|SetHealth (- (Variables|Default|GetHealth) Damage))
  (if (<= (Variables|Default|GetHealth) 0.0)
    (Class|EnemyBase|SpawnDrops "/Game/Data/Enemy/DT_EnemyDataTable.DT_EnemyDataTable" (Variables|Default|GetRowName) 1e+02)
    (bind _returnvalue (Actor|GetActorOfClass "/Game/External_Asset/Enemy/Blueprint/BP_PoolManager.BP_PoolManager_C"))
    (Default|ReturnEnemy _returnvalue self "NewEnumerator5")))

(fn ConstructionScript)