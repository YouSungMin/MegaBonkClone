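; BP_EnemySpawnerMulti is an enemy spawner that periodically places a random enemy type from its list at its own location.
; On BeginPlay it finds the level's BP_PoolManager and starts a looping timer at the spawn interval.
; Each tick of that timer requests a random NewEnemyList entry from the pool, then moves the returned enemy to the spawner, with validity checks on both manager and enemy.
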(event Custom|SpawnMob
  (Variables|Default|GetPoolManager
    (:then
      (bind _enemyactor (Default|GetEnemy (Variables|Default|GetPoolManager) (.OutItem (Utilities|Array|Random (Variables|Default|GetNewEnemyList)))))
      (Utilities|IsValid 0
        (:Is%20Valid
          (Transformation|SetActorLocation _enemyactor (Transformation|GetActorLocation) false false))))
    (:else)))

(event EventBeginPlay
  (bind _returnvalue (Actor|GetActorOfClass "/Game/External_Asset/Enemy/Blueprint/BP_PoolManager.BP_PoolManager_C"))
  (Variables|Default|SetPoolManager _returnvalue)
  (Utilities|Time|SetTimerbyEvent (delegate Custom|SpawnMob) (Variables|Default|GetSpawnInterval) true))

(fn ConstructionScript)