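; BP_2Slime is a slime enemy that chases the player and deals contact damage.
; On BeginPlay it reads the Slime row of DT_EnemyDataTable for speed and health, adding a bonus derived from its Time variable.
; MoveSlime re-issues AIMoveTo after each success or failure.
; Any sphere overlap damages the player by AttackPower, and death destroys the slime and decrements its Spawner's EnemyNumber.
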(event OnComponentBeginOverlap(Sphere)
  (params (OverlappedComponent :type Primitive%20Component%20Object%20Reference) (OtherActor :type Actor%20Object%20Reference) (OtherComp :type Primitive%20Component%20Object%20Reference) (OtherBodyIndex :type Integer) (bFromSweep :type Boolean) (SweepResult :type Hit%20Result%20Structure%20%28by%20ref%29))
  (bind _asbp_character_base (Utilities|Casting|CastToBP_CharacterBase (Game|GetPlayerCharacter 0)))
  (Game|Damage|ApplyDamage _asbp_character_base (.attackpower (stale EventBeginPlay _returnvalue)) 0 0))

(event Custom|MoveSlime
  (AI|AIMoveTo self "0, 0, 0" (Game|GetPlayerCharacter 0) 5.0 false
    (:OnSuccess
      (Utilities|FlowControl|Delay 0.2)
      (CallFunction|MoveSlime))
    (:OnFail
      (Utilities|FlowControl|Delay 0.2)
      (CallFunction|MoveSlime))))

(event EventBeginPlay
  (bind _returnvalue (Utilities|GetDataTableRow "/Game/Data/Enemy/DT_EnemyDataTable.DT_EnemyDataTable" "Slime")
    (:then
      (CallFunction|MoveSlime)
      (Variables|Default|SetHealth (+ (.maxhp _returnvalue) (/ (+ (Variables|Default|GetTime) (Utilities|Time|GetWorldDeltaSeconds)) 1e+01)))
      (Variables|/Script/Engine.CharacterMovementComponent|SetMaxWalkSpeed (Variables|Character|GetCharacterMovement) (.movespeed _returnvalue)))))

(event Game|Damage|EventAnyDamage
  (params (Damage :type Float%20%28single-precision%29) (DamageType :type Damage%20Type%20Object%20Reference) (InstigatedBy :type Controller%20Object%20Reference) (DamageCauser :type Actor%20Object%20Reference))
  (bind _spawner (Variables|Default|GetSpawner))
  (Variables|Default|SetHealth (- (Variables|Default|GetHealth) Damage))
  (if (<= (Variables|Default|GetHealth) 0.0)
    (Actor|DestroyActor)
    (Variables|/Game/External_Asset/Enemy/Blueprint/BP_EnemySpawner.BP_EnemySpawner_C|SetEnemyNumber _spawner (- (Variables|/Game/External_Asset/Enemy/Blueprint/BP_EnemySpawner.BP_EnemySpawner_C|GetEnemyNumber _spawner) 1.0))))

(fn ConstructionScript)