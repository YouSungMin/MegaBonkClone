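; Enemy spawner actor that places enemies at random reachable navmesh points around itself, with a cap that grows over elapsed time.
; Tick accumulates time and raises the cap, while a looping one-second timer spawns when the count is below it.
; Early spawns are BP_1Goblin, later switching to BP_Enemy.
; Only goblin spawns increment the count, and nothing here decrements it.
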(event Custom|SpawnEnemy
  (if (> (Variables|Default|GetEnemyMax) (Variables|Default|GetEnemyNumber))
    (Utilities|FlowControl|Sequence
      (:then_0
        (if (>= (Variables|Default|GetTime) 0.0)
          (if (< (Variables|Default|GetTime) 1e+01)
            (CallFunction|SpawnGoblin))))
      (:then_1
        (if (>= (Variables|Default|GetTime) 1e+01)
          (CallFunction|SpawnTestEnemy))))))

(event Custom|SpawnGoblin
  (Game|SpawnActorfromClass "/Game/External_Asset/Enemy/Blueprint/BP_1Goblin.BP_1Goblin_C" (Math|Transform|MakeTransform (.RandomLocation (AI|Navigation|GetRandomReachablePointinRadius (Transformation|GetActorLocation) 7e+03 0 0)) "0, 0, 0" "1.000000,1.000000,1.000000") "Undefined" "MultiplyWithRoot" 0 0)
  (Variables|Default|SetEnemyNumber (+ (Variables|Default|GetEnemyNumber) 1.0))
  (Development|PrintString "Hello"))

(event Custom|SpawnTestEnemy
  (Game|SpawnActorfromClass "/Game/External_Asset/Enemy/Blueprint/BP_Enemy.BP_Enemy_C" (Math|Transform|MakeTransform (.RandomLocation (AI|Navigation|GetRandomReachablePointinRadius (Transformation|GetActorLocation) 7e+03 0 0)) "0, 0, 0" "1.000000,1.000000,1.000000") "Undefined" "MultiplyWithRoot" 0 0)
  (Variables|Default|SetEnemyNumber (+ (Variables|Default|GetEnemyNumber) 0.0))
  (Development|PrintString "Hello"))

(event EventBeginPlay
  (Utilities|Time|SetTimerbyEvent (delegate Custom|SpawnEnemy) 1.0 true))

(event EventTick
  (params (DeltaSeconds :type Float%20%28single-precision%29))
  (Variables|Default|SetEnemyMax (+ 3.0 (/ (Variables|Default|GetTime) 5.0)))
  (Variables|Default|SetTime (+ (Variables|Default|GetTime) DeltaSeconds)))

(fn ConstructionScript)