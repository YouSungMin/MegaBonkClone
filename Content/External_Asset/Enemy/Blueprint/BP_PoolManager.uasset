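; Enemy pool manager actor that pre-spawns ten enemies per class at random reachable points around itself and supplies them by type.
; GetEnemy activates and repositions pooled enemies, or spawns new ones when empty, while the active count is under a limit.
; ReturnEnemy deactivates enemies and stores them in the per-type map, though it always reads the first enum entry's array.
; A looping timer periodically raises the active limit up to a cap.
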(event Custom|IncreaseLimit
  (Variables|Default|SetMaxEnemyLimit (Math|Integer|Clamp(Integer) (+ (Variables|Default|GetMaxEnemyLimit) (Variables|Default|GetLimitIncreaseRate)) 0 100)))

(event EventBeginPlay
  (Utilities|Time|SetTimerbyEvent (delegate Custom|IncreaseLimit) 15.0 true)
  (bind _keys (Utilities|Map|Keys (Variables|Default|GetEnemyClasses)))
  (for _array_element _keys
    (for _index (range 0 9)
      (bind _returnvalue (Game|SpawnActorfromClass (.Value (Utilities|Map|Find (Variables|Default|GetEnemyClasses) _array_element)) (Math|Transform|MakeTransform (+ (.RandomLocation (AI|Navigation|GetRandomReachablePointinRadius (Transformation|GetActorLocation) 7e+03 0 0)) "0.000000,0.000000,100.000000") "0, 0, 0" "1.000000,1.000000,1.000000") "AdjustIfPossibleButAlwaysSpawn" "MultiplyWithRoot" 0 0))
      (CallFunction|ReturnEnemy _returnvalue _array_element))))

(fn ConstructionScript)

(fn GetEnemy
  (params (Type :type E_EnemyType%20Enum :default "NewEnumerator0"))
  (bind _poolstorage (Variables|Default|GetPoolStorage))
  (bind _value (Utilities|Map|Find _poolstorage Type))
  (bind _enemyarray (Utilities|Struct|BreakS_EnemyArray _value))
  (bind _returnvalue (Utilities|Array|LastIndex _enemyarray))
  (bind _output (Utilities|Array|Get(acopy) _enemyarray _returnvalue))
  (Development|PrintString (Utilities|String|ToString(Integer) (Variables|Default|GetActivateEnemyCount)))
  (if (< (Variables|Default|GetActivateEnemyCount) (Variables|Default|GetMaxEnemyLimit))
    (if (> (Utilities|Array|Length _enemyarray) 0)
      (Utilities|Array|RemoveIndex _enemyarray _returnvalue)
      (Class|BPIPoolable|OnActivate(Message) _output)
      (Transformation|SetActorTransform _output (Math|Transform|MakeTransform (+ (.RandomLocation (AI|Navigation|GetRandomReachablePointinRadius (Transformation|GetActorLocation) 7e+03 0 0)) "0.000000,0.000000,100.000000") "0, 0, 0" "1.000000,1.000000,1.000000") false true)
      (Variables|Default|SetActivateEnemyCount (+ (Variables|Default|GetActivateEnemyCount) 1))
      (return (stale _returnvalue_2))
      (else
        (bind _returnvalue_2 (Game|SpawnActorfromClass (.Value (Utilities|Map|Find (Variables|Default|GetEnemyClasses) Type)) (Math|Transform|MakeTransform (+ (.RandomLocation (AI|Navigation|GetRandomReachablePointinRadius (Transformation|GetActorLocation) 7e+03 0 0)) "0.000000,0.000000,100.000000") "0, 0, 0" "1.000000,1.000000,1.000000") "AdjustIfPossibleButAlwaysSpawn" "MultiplyWithRoot" 0 0))
        (Variables|Default|SetActivateEnemyCount (+ (Variables|Default|GetActivateEnemyCount) 1))
        (return 0)))))

(fn ReturnEnemy
  (params (EnemyActor :type Actor%20Object%20Reference) (Type :type E_EnemyType%20Enum :default "NewEnumerator0"))
  (bind _poolstorage (Variables|Default|GetPoolStorage))
  (bind _value (Utilities|Map|Find _poolstorage "NewEnumerator0"))
  (bind _enemyarray (Utilities|Struct|BreakS_EnemyArray _value))
  (Variables|Default|SetActivateEnemyCount (Math|Integer|Clamp(Integer) (- (Variables|Default|GetActivateEnemyCount) 1) 0 1000))
  (Class|BPIPoolable|OnDeactivate(Message) EnemyActor)
  (Utilities|Array|Add _enemyarray EnemyActor)
  (Utilities|Map|Add (Variables|Default|GetPoolStorage) Type (Utilities|Struct|MakeS_EnemyArray false _enemyarray)))