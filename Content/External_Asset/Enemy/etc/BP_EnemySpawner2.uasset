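; BP_EnemySpawner2 is an enemy spawner that periodically brings pooled enemies to its own location.
; On BeginPlay it finds the BP_PoolManager in the level and starts a looping timer at SpawnInterval.
; Each tick of that timer picks a random key from the manager's EnemyClasses map, requests an enemy through GetEnemy and moves it to the spawner without sweeping.
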(event Custom|SpawnMob
  (bind _poolmanager (Variables|Default|GetPoolManager))
  (Variables|Default|GetPoolManager
    (:then
      (bind _keys (Utilities|Map|Keys (Variables|/Game/External_Asset/Enemy/Blueprint/BP_PoolManager.BP_PoolManager_C|GetEnemyClasses _poolmanager)))
      (bind _enemyactor (Default|GetEnemy _poolmanager (.OutItem (Utilities|Array|Random _keys))))
      (Utilities|IsValid 0
        (:Is%20Valid
          (Transformation|SetActorLocation _enemyactor (Transformation|GetActorLocation) false false))))
    (:else)))

(event EventBeginPlay
  (bind _returnvalue (Actor|GetActorOfClass "/Game/External_Asset/Enemy/Blueprint/BP_PoolManager.BP_PoolManager_C"))
  (Variables|Default|SetPoolManager _returnvalue)
  (Utilities|Time|SetTimerbyEvent (delegate Custom|SpawnMob) (Variables|Default|GetSpawnInterval) true))

(fn ConstructionScript)